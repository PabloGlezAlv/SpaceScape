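; BP_Drawer is an interactable piece of furniture that the player walks into and out of, toggled by InsideDrawer.
; Entering drives movement input toward RefIn, then swings the door shut; exiting swings it open, then drives the player toward RefOut, each with a door sound.
; Chained timelines time the walk and door rotation, with InAnimation set on BP_FirstPersonCharacter until the sequence finishes.
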(event `self.ReceiveBeginPlay`)

(event `/Game/BluePrints/BPI_Interaction.Interact`
  (bind _returnvalue (`GameplayStatics.GetPlayerCharacter` 0))
  (bind _returnvalue_location (`KismetMathLibrary.BreakTransform` (`SceneComponent.K2_GetComponentToWorld` (`self.RefOut`))))
  (bind _returnvalue_location_2 (`KismetMathLibrary.BreakTransform` (`SceneComponent.K2_GetComponentToWorld` (`self.RefIn`))))
  (set `self.StartPosition` (`self.K2_GetActorLocation` _returnvalue))
  (set `self.StartRotation` (`self.K2_GetActorRotation` _returnvalue))
  (bind _asbp_first_person_character (cast `/Game/FirstPerson/Blueprints/BP_FirstPersonCharacter` (`GameplayStatics.GetPlayerCharacter` 0))
    (:`then`
      (set `/Game/FirstPerson/Blueprints/BP_FirstPersonCharacter.InAnimation` true _asbp_first_person_character)
      (if (not (`self.insideDrawer`))
        (set `self.insideDrawer` true)
        (`Timeline|PositionPlayer` :!via `PlayFromStart`
          (:`Update`
            (`Pawn.AddMovementInput` (`GameplayStatics.GetPlayerCharacter` 0) (`KismetMathLibrary.Normal` (- _returnvalue_location_2 (`self.StartPosition`))) 1.0 false))
          (:`Finished`
            (`GameplayStatics.PlaySoundAtLocation` "/Game/Sounds/Door.Door" (`SceneComponent.K2_GetComponentLocation` (`self.Door`)) (struct) 1.0 1.0 0.0 null null null null)
            (bind (_direction _doorfloat) (`Timeline|CloseDoor`)
              (:`Update`
                (`SceneComponent.K2_SetRelativeRotation` (`self.Door`) (`KismetMathLibrary.MakeRotator` 0.0 0.0 (`KismetMathLibrary.Lerp` 100.0 0.0 _doorfloat)) false false))
              (:`Finished`
                (bind _asbp_first_person_character_2 (cast `/Game/FirstPerson/Blueprints/BP_FirstPersonCharacter` (`GameplayStatics.GetPlayerCharacter` 0)))
                (set `/Game/FirstPerson/Blueprints/BP_FirstPersonCharacter.InAnimation` false _asbp_first_person_character_2)))))
        (else
          (set `self.insideDrawer` false)
          (`GameplayStatics.PlaySoundAtLocation` "/Game/Sounds/Door.Door" (`SceneComponent.K2_GetComponentLocation` (`self.Door`)) (struct) 1.0 1.0 0.0 null null null null)
          (bind (_direction_2 _doorfloat_2) (`Timeline|Timeline` :!via `PlayFromStart`)
            (:`Update`
              (`SceneComponent.K2_SetRelativeRotation` (`self.Door`) (`KismetMathLibrary.MakeRotator` 0.0 0.0 (`KismetMathLibrary.Lerp` 0.0 100.0 _doorfloat_2)) false false))
            (:`Finished`
              (`Timeline|Timeline_0` :!via `PlayFromStart`
                (:`Update`
                  (`Pawn.AddMovementInput` (`GameplayStatics.GetPlayerCharacter` 0) (`KismetMathLibrary.Normal` (- _returnvalue_location (`self.StartPosition`))) 1.0 false))
                (:`Finished`
                  (bind _asbp_first_person_character_3 (cast `/Game/FirstPerson/Blueprints/BP_FirstPersonCharacter` (`GameplayStatics.GetPlayerCharacter` 0)))
                  (set `/Game/FirstPerson/Blueprints/BP_FirstPersonCharacter.InAnimation` false _asbp_first_person_character_3))))))))
    (:`CastFailed`
      (`KismetSystemLibrary.PrintString` "Cast Failed"))))

(fn `UserConstructionScript`)