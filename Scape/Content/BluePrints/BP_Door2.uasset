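; BP_Door2 is a locked door that swings open when the player interacts with it while holding the key.
; Interact casts the player character to BP_FirstPersonCharacter and checks its Key variable, with an Opening flag allowing only one opening.
; Opening disables the Door's collision and plays a timeline that lerps the DoorPoint pivot's relative yaw; nothing closes it again.
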(event `/Game/BluePrints/BPI_Interaction.Interact`
  (bind _asbp_first_person_character (cast `/Game/FirstPerson/Blueprints/BP_FirstPersonCharacter` (`GameplayStatics.GetPlayerCharacter` 0)))
  (if (`/Game/FirstPerson/Blueprints/BP_FirstPersonCharacter.Key` _asbp_first_person_character)
    (if (not (`self.opening`))
      (set `self.opening` true)
      (`PrimitiveComponent.SetCollisionEnabled` (`self.Door`) "NoCollision")
      (bind (_direction _doorfloat) (`Timeline|Timeline` :!via `PlayFromStart`)
        (:`Update`
          (`SceneComponent.K2_SetRelativeRotation` (`self.DoorPoint`) (`KismetMathLibrary.MakeRotator` 0.0 0.0 (`KismetMathLibrary.Lerp` 0.0 100.0 _doorfloat)) false false))))))

(fn `UserConstructionScript`)